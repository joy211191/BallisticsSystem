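; Projectile actor for a ballistics system that bends its flight using world X and Y speeds read from the custom game instance.
; On BeginPlay it caches both speeds, and every Tick it adds them plus a fixed gravity-like downward term to the ProjectileMovement velocity.
; The addition is not scaled by delta time, so the trajectory depends on frame rate.
; Tick also prints both speeds on screen as debug output.
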(event EventBeginPlay
  (bind _ascustom_game_instance (Utilities|Casting|CastToCustomGameInstance (Game|GetGameInstance)))
  (Variables|Default|SetWorldYSpeed (Variables|/Game/Blueprints/CustomGameInstance.CustomGameInstance_C|GetYSpeed _ascustom_game_instance))
  (Variables|Default|SetWorldXSpeed (Variables|/Game/Blueprints/CustomGameInstance.CustomGameInstance_C|GetXSpeed _ascustom_game_instance)))

(event Collision|EventActorBeginOverlap
  (params (OtherActor :type Actor%20Object%20Reference)))

(event EventTick
  (params (DeltaSeconds :type Float%20%28single-precision%29))
  (bind _projectilemovement (Variables|Default|GetProjectileMovement))
  (bind _worldyspeed (Variables|Default|GetWorldYSpeed))
  (bind _worldxspeed (Variables|Default|GetWorldXSpeed))
  (Variables|/Script/Engine.MovementComponent|SetVelocity _projectilemovement (+ (Variables|/Script/Engine.MovementComponent|GetVelocity _projectilemovement) (Math|Vector|MakeVector _worldxspeed _worldyspeed -9.81)))
  (Development|PrintString (Utilities|String|ToString(Float) _worldxspeed) true true "(R=1.000000,G=0.048397,B=0.000000,A=1.000000)")
  (Development|PrintString (Utilities|String|ToString(Float) _worldyspeed) true true "(R=0.000000,G=1.000000,B=0.022884,A=1.000000)"))

(fn ConstructionScript)